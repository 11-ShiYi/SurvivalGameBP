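; Survival game mode that handles game start, restart, game over and quitting.
; On BeginPlay it caches the game instance, Cabinet and GlobalTimer, then creates the runtime UI.
; Game over stops the timer and shows the failed panel with survival time and a record message.
; CheckScore compares total hours against the BestScore save, overwrites it on a new record, and labels the current run's time "longest" when falling short.
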(event `self.ReceiveBeginPlay`
  (`|ExecutionSequence`
    (:`then_0`
      (set `self.GameInstance` (cast `/Game/Blueprints/SurvivalGameInstance` (`GameplayStatics.GetGameInstance`) :!pure true)))
    (:`then_1`
      (bind _outactors (`GameplayStatics.GetAllActorsOfClass` "/Game/Blueprints/Props/Cabinet.Cabinet_C"))
      (set `self.Cabinet` (`|GetArrayItem` _outactors)))
    (:`then_2`
      (bind _outactors_2 (`GameplayStatics.GetAllActorsOfClass` "/Game/Blueprints/GlobalTimer.GlobalTimer_C"))
      (set `self.GlobalTimer` (`|GetArrayItem` _outactors_2))
      (`/Game/Blueprints/SurvivalGameInstance.CreateRuntimeUI` (`self.GameInstance`)))))

(event `RestartGame`
  (`GameplayStatics.OpenLevel` "MainLevel"))

(event `GameOver`
  (bind _gameinstance (`self.GameInstance`))
  (bind _globaltimer (`self.GlobalTimer`))
  (bind _currentday (`/Game/Blueprints/GlobalTimer.CurrentDay` _globaltimer))
  (bind _currenthour (`/Game/Blueprints/GlobalTimer.CurrentHour` _globaltimer))
  (`/Game/Blueprints/GlobalTimer.StopTimer` (`self.GlobalTimer`))
  (`/Game/Blueprints/SurvivalGameInstance.HIdeAllPanels` _gameinstance)
  (`/Game/Blueprints/SurvivalGameInstance.ShowFailedPanel` _gameinstance)
  (bind _recordtext (`self.Check Score` _currentday _currenthour))
  (`/Game/UI/UI_Failed.SetTexts` (`/Game/Blueprints/SurvivalGameInstance.FailedPanel` _gameinstance) _currentday _currenthour (`KismetTextLibrary.Conv_StringToText` _recordtext)))

(event `QuitGame`
  (`KismetSystemLibrary.ExecuteConsoleCommand` "exit" null))

(fn `Check Score`
  (params (NewDay :type Integer) (NewHour :type Integer))
  (returns (RecordText :type String))
  (bind _returnvalue (`GameplayStatics.DoesSaveGameExist` "BestScore"))
  (if _returnvalue
    (bind _returnvalue_2 (`GameplayStatics.LoadGameFromSlot` "BestScore"))
    (bind _asbest_score (cast `/Game/Blueprints/BestScore` _returnvalue_2))
    (bind _returnvalue_3 (- (+ (* NewDay 24) NewHour) (+ (* (`/Game/Blueprints/BestScore.BestDay` _asbest_score) 24) (`/Game/Blueprints/BestScore.BestHour` _asbest_score))))
    (if (> _returnvalue_3 0)
      _
      (elif (== _returnvalue_3 0)
        (return "加油，离打破记录只差一步之遥！")
        (else
          (return (`KismetStringLibrary.Concat_StrStr` "最长生存时间：" (`KismetStringLibrary.Conv_IntToString` NewDay) "天" (`KismetStringLibrary.Conv_IntToString` NewHour) "小时"))))))
  (bind _returnvalue_4 (`GameplayStatics.CreateSaveGameObject` "/Game/Blueprints/BestScore.BestScore_C"))
  (set `/Game/Blueprints/BestScore.BestDay` NewDay _returnvalue_4)
  (set `/Game/Blueprints/BestScore.BestHour` NewHour _returnvalue_4)
  (`GameplayStatics.SaveGameToSlot` _returnvalue_4 "BestScore")
  (return "恭喜你创造了新纪录！"))

(fn `UserConstructionScript`)